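; BP_Waves_Gate is a wave-mode gate that destroys spawned pawns entering its box and counts down toward a loss.
; On each pawn overlap it rebuilds the target list from every BP_SplineSpawner's spawned pawns.
; A matching pawn decrements CountForLose and refreshes the text render; at zero it can optionally stop all spawners.
; The construction script sizes the box from BoxExtent and initializes the counter text.
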(event `self.Box.OnComponentBeginOverlap`
  (params (OverlappedComponent :type "PrimitiveComponent Object Reference") (OtherActor :type "Actor Object Reference") (OtherComp :type "PrimitiveComponent Object Reference") (OtherBodyIndex :type Integer) (bFromSweep :type Boolean) (SweepResult :type "HitResult Structure (by ref)"))
  (bind _aspawn (cast `Pawn` OtherActor))
  (`self.-GetAllSpawnedActors`)
  (if (`KismetArrayLibrary.Array_Contains` (`self.TargetsPawns`) _aspawn)
    (`self.K2_DestroyActor` OtherActor)
    (bind _output_get (set `self.CountForLose` (`KismetMathLibrary.Max` (- (`self.CountForLose`) 1))))
    (`self.-UpdateText`)
    (if (== _output_get 0)
      (if (`self.StopAllSpawnerIfLose`)
        (`self.-StopAllSpawners`))
      (else
        (`self.-GetAllSpawnedActors`)))))

(fn `-GetAllSpawnedActors`
  (`KismetArrayLibrary.Array_Clear` (`self.TargetsPawns`))
  (bind _outactors (`GameplayStatics.GetAllActorsOfClass` "/Game/AdvancedUniversalSpawner/BP_SplineSpawner.BP_SplineSpawner_C"))
  (for _array_element _outactors
    (for _array_element_2 (`/Game/AdvancedUniversalSpawner/BP_SplineSpawner.SpawnedPawns` _array_element)
      (`KismetArrayLibrary.Array_Add` (`self.TargetsPawns`) (`.PawnRef_5_C1A9AF2E4ABC0AFBC058BC82EFDF5214` (break `/Game/AdvancedUniversalSpawner/Data/Str/Str_Pawn_Info` _array_element_2))))))

(fn `-StopAllSpawners`
  (bind _outactors (`GameplayStatics.GetAllActorsOfClass` "/Game/AdvancedUniversalSpawner/BP_SplineSpawner.BP_SplineSpawner_C"))
  (for _array_element _outactors
    (`/Game/AdvancedUniversalSpawner/BP_SplineSpawner.-StopSpawning` _array_element)))

(fn `-UpdateText`
  (`TextRenderComponent.K2_SetText` (`self.TextRender`) (`|FormatText` "Count For Lose - {Num}" (`KismetMathLibrary.Max` (`self.CountForLose`)))))

(fn `UserConstructionScript`
  (`BoxComponent.SetBoxExtent` (`self.Box`) (`self.BoxExtent`) true)
  (`self.-UpdateText`))